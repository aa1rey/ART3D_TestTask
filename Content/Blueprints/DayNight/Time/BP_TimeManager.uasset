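; BP_TimeManager drives the day/night look by moving the sun and refreshing the sky sphere from a time-of-day value.
; UpdateAll wraps Time in seconds to a 24-hour value, then samples float curves for the directional light's pitch and intensity.
; It then updates the Sky Sphere's sun direction to match.
; On BeginPlay, it finds every BP_Lamp and binds an event to OnDayEnd for each.
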(event `self.ReceiveBeginPlay`
  (`parent.ReceiveBeginPlay`)
  (bind _outactors (`GameplayStatics.GetAllActorsOfClass` "/Game/Blueprints/DayNight/BP_Lamp.BP_Lamp_C"))
  (for _array_element _outactors
    (add `self.OnDayEnd` (`|CreateDelegate` _array_element :!event `DayBeginEnd`))))

(event `self.UpdateAll`
  (params (CurrHour :type "Float (single-precision)"))
  ;[0 0 0] Dir light position
  (`self.K2_SetActorRotation` (`self.Sun`) (`KismetMathLibrary.MakeRotator` 0.0 (`CurveFloat.GetFloatValue` (`self.DirLightPitch`) (/ (mod (`self.Time`) 86400.0) 3600.0))) false)
  ;[0 0 0] Dir light intensity
  (`LightComponent.SetIntensity` (`Light.LightComponent` (`self.Sun`)) (`CurveFloat.GetFloatValue` (`self.DirLightIntensity`) (/ (mod (`self.Time`) 86400.0) 3600.0)))
  ;[0 0 0] Update Sky Sphere
  (`/Engine/EngineSky/BP_Sky_Sphere.UpdateSunDirection` (`self.SkySphere`)))

(fn `UserConstructionScript`
  (`parent.UserConstructionScript`))