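; BP_HUD_Cubes is a HUD Blueprint that connects a cube color-picking UI to the cube manager in the level.
; On BeginPlay it finds the first BP_CubeManager and, if one exists, creates WBP_ChangeCubeColor with the manager's cube count, showing the cursor in Game and UI input mode.
; It binds the widget's selection events, forwarding cube selection and chosen color properties to the manager to update that cube's widget and color.
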(event `self.ReceiveBeginPlay`
  (bind _outactors (`GameplayStatics.GetAllActorsOfClass` "/Game/Blueprints/CubeMovement/BP_CubeManager.BP_CubeManager_C"))
  (if (!= (`KismetArrayLibrary.Array_Length` _outactors) 0)
    (set `self.CubeManagerRef` (`|GetArrayItem` _outactors))
    (`self.CreateWidget`)))

(event `CreateWidget`
  (bind _returnvalue (`|CreateWidget` "/Game/Blueprints/UI/Cubes/WBP_ChangeCubeColor.WBP_ChangeCubeColor_C" (`GameplayStatics.GetPlayerController` 0) (`CubeManager.CubesAmount` (`self.CubeManagerRef`))))
  (bind _output_get (set `self.Widget` _returnvalue))
  (`UserWidget.AddToViewport` _output_get 9999)
  (add `/Game/Blueprints/UI/Cubes/WBP_ChangeCubeColor.OnAllPropertiesSelected` (`self.Widget`) (delegate `OnAllPropertiesSelected_Event`))
  (add `/Game/Blueprints/UI/Cubes/WBP_ChangeCubeColor.OnCubeSelected` (`self.Widget`) (delegate `OnCubeSelected_Event`))
  (set `PlayerController.bShowMouseCursor` true (`GameplayStatics.GetPlayerController` 0))
  (`WidgetBlueprintLibrary.SetInputMode_GameAndUIEx` (`GameplayStatics.GetPlayerController` 0) null "DoNotLock" false))

(event `OnAllPropertiesSelected_Event`
  (params (Index :type Integer) (CubeColor :type "ECubeColor Enum" :default "White") (LinearColor :type "LinearColor Structure"))
  (`CubeManager.UpdateCubeColorByIndex` (`self.CubeManagerRef`) Index CubeColor LinearColor))

(event `OnCubeSelected_Event`
  (params (CurrentIndex :type Integer))
  (`/Game/Blueprints/CubeMovement/BP_CubeManager.UpdateCubeWidget` (`self.CubeManagerRef`) CurrentIndex))

(fn `UserConstructionScript`)