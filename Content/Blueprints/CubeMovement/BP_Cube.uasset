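; BP_Cube is a cube Blueprint with a widget component that hosts a WBP_CubeInfo info display.
; On BeginPlay it casts the component's widget to WBP_CubeInfo and binds to the OnColorUpdate event dispatcher.
; UpdateWidgetInfo broadcasts a color through that dispatcher, and SetWidgetVisible toggles the widget between SelfHitTestInvisible and Hidden.
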(event `self.ReceiveBeginPlay`
  (`parent.ReceiveBeginPlay`)
  (bind _aswbp_cube_info (cast `/Game/Blueprints/UI/Cubes/WBP_CubeInfo` (`WidgetComponent.GetWidget` (`self.Widget`))))
  (add `self.OnColorUpdate` (`|CreateDelegate` _aswbp_cube_info :!event `UpdateColor`)))

(event `self.SetWidgetVisible`
  (params (bNewVisible :type Boolean))
  (`Widget.SetVisibility` (`WidgetComponent.GetWidget` (`self.Widget`)) (select `bool` bNewVisible :`false` "Hidden" :`true` "SelfHitTestInvisible" :!type "ESlateVisibility Enum")))

(event `self.UpdateWidgetInfo`
  (params (Color :type "ECubeColor Enum" :default "White"))
  (`self.OnColorUpdate` Color))

(fn `UserConstructionScript`)